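; JamDamagable is a Blueprint that gives its owner basic health and death handling.
; Damage subtracts an amount from Health only while it is still alive, then fires the OnDead dispatcher once Health drops to zero or below.
; IsDead derives the death state directly from Health, so further hits after death are ignored.
; The event graph is empty, and a debug damage print is left disconnected.
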(event EventBeginPlay)

(event EventTick
  (params (DeltaSeconds :type Float%20%28single-precision%29)))

(fn IsDead
  (return (<= (Variables|Default|GetHealth) 0.0)))

(fn Damage
  (params (Amount :type Float%20%28single-precision%29))
  (if (not (CallFunction|IsDead))
    (bind _output_get (Variables|Default|SetHealth (- (Variables|Default|GetHealth) Amount)))
    (if (CallFunction|IsDead)
      (Default|CallOnDead))))