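; Behavior Tree task that waits until the AI's pawn has a clear line of sight to the enemy stored in the Blackboard.
; Each tick it runs a Visibility trace from the enemy to the pawn, ignoring both and drawing debug for one frame.
; An unblocked trace finishes with success, a blocked one keeps the task running, and a failed controller or enemy cast finishes with failure.
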(event EventTick
  (params (OwnerActor :type Actor%20Object%20Reference) (DeltaSeconds :type Float%20%28single-precision%29))
  (bind _asaicontroller (Utilities|Casting|CastToAIController OwnerActor)
    (:then
      (bind _asactor (Utilities|Casting|CastToActor (AI|Components|Blackboard|GetValueasObject (AI|GetBlackboard _asaicontroller) (Variables|Default|GetEnemyKey)))
        (:then
          (bind _returnvalue (Collision|LineTraceByChannel (Transformation|GetActorLocation _asactor) (Transformation|GetActorLocation (Pawn|GetControlledPawn _asaicontroller)) "TraceTypeQuery1" false (Utilities|Array|MakeArray _asactor (Pawn|GetControlledPawn _asaicontroller)) "ForOneFrame"))
          (if (not _returnvalue)
            (AI|BehaviorTree|FinishExecute true)))
        (:CastFailed
          (AI|BehaviorTree|FinishExecute false :!label _label))))
    (:CastFailed
      (goto _label))))