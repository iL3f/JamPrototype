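; JamAiController is an AI controller for enemies that hunt the player's JamCharacter.
; On BeginPlay it sets up EnemyBlackboard and runs the EnemyBehaviour behavior tree.
; AI perception updates write a sensed JamCharacter to the blackboard's enemy key and clear it when any stimulus is lost.
; OnDied stops the brain component's logic.
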(event OnTargetPerceptionUpdated(AIPerception)
  (params (Actor :type Actor%20Object%20Reference) (Stimulus :type AI%20Stimulus%20Structure))
  (if (.bsuccessfullysensed Stimulus)
    (bind _asjam_character (Utilities|Casting|CastToJamCharacter Actor))
    (CallFunction|SetEnemy _asjam_character)
    (else
      (CallFunction|SetEnemy))))

(event EventBeginPlay
  (Class|AIController|UseBlackboard "/Game/Blueprints/AI/EnemyBlackboard.EnemyBlackboard")
  (AI|RunBehaviorTree "/Game/Blueprints/AI/EnemyBehaviour.EnemyBehaviour"))

(event EventTick
  (params (DeltaSeconds :type Float%20%28single-precision%29)))

(fn ConstructionScript)

(fn SetEnemy
  (params (Enemy :type Character%20Object%20Reference))
  (AI|Components|Blackboard|SetValueasObject (AI|GetBlackboard 0) (Variables|Default|GetEnemyKey) Enemy))

(fn OnDied
  (AI|Logic|StopLogic (Variables|Default|GetBrainComponent) "death"))