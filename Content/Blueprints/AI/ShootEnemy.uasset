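; Behavior tree task that makes a JamEnemyCharacter fire a burst of shots.
; On execute it gets the controlled pawn and starts a looping timer at the fire rate, calling Shoot on each tick until the burst count runs out.
; It then clears the timer and finishes successfully; abort also clears the timer.
; A non-controller owner fails the task, while a failed pawn cast never finishes it.
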(event Custom|Fire
  (Default|Shoot (Variables|Default|GetChar))
  (bind _result (Math|Integer|DecrementInt (Variables|Default|GetCount))
    (:%20%20
      (if (<= _result 0)
        (Utilities|Time|ClearandInvalidateTimerbyHandle (Variables|Default|GetTimer))
        (AI|BehaviorTree|FinishExecute true)))))

(event EventReceiveExecute
  (params (OwnerActor :type Actor%20Object%20Reference))
  (bind _ascontroller (Utilities|Casting|CastToController OwnerActor)
    (:then
      (bind _asjam_enemy_character (Utilities|Casting|CastToJamEnemyCharacter (Pawn|GetControlledPawn _ascontroller)))
      (Variables|Default|SetChar _asjam_enemy_character)
      (bind _returnvalue (Utilities|Time|SetTimerbyEvent (delegate Custom|Fire) (/ 1.0 (Variables|Default|GetFireRate)) true))
      (Variables|Default|SetTimer _returnvalue)
      (Variables|Default|SetCount (Variables|Default|GetBurstSize)))
    (:CastFailed
      (AI|BehaviorTree|FinishExecute false))))

(event EventReceiveAbort
  (params (OwnerActor :type Actor%20Object%20Reference))
  (Utilities|Time|ClearandInvalidateTimerbyHandle (Variables|Default|GetTimer)))