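; Automatic double sliding door that opens while actors overlap it and closes when they leave.
; Begin and end overlap events call Open and Close, which set opposite X offset targets for the Left and Right components.
; A counter tracks overlaps so the door only closes when the count returns to zero.
; Tick continuously eases both panels toward their targets with VInterpTo at the open speed.
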(event EventTick
  (params (DeltaSeconds :type Float%20%28single-precision%29))
  (bind _left (Variables|Default|GetLeft))
  (bind _right (Variables|Default|GetRight))
  (Transformation|SetRelativeLocation _left (Math|Interpolation|VInterpTo (Variables|/Script/Engine.SceneComponent|GetRelativeLocation _left) (Math|Vector|MakeVector (Variables|Default|GetLeftPosOffset) 0.0 0.0) DeltaSeconds (Variables|Default|GetOpenSpeed)) false false)
  (Transformation|SetRelativeLocation _right (Math|Interpolation|VInterpTo (Variables|/Script/Engine.SceneComponent|GetRelativeLocation _right) (Math|Vector|MakeVector (Variables|Default|GetRightPosOffset) 0.0 0.0) DeltaSeconds (Variables|Default|GetOpenSpeed)) false false))

(event Collision|EventActorBeginOverlap
  (params (OtherActor :type Actor%20Object%20Reference))
  (CallFunction|Open))

(event Collision|EventActorEndOverlap
  (params (OtherActor :type Actor%20Object%20Reference))
  (CallFunction|Close))

(fn ConstructionScript)

(fn Open
  (bind _openoffset (Variables|Default|GetOpenOffset))
  (Math|Integer|IncrementInt (Variables|Default|GetOpenCounter)
    (:%20%20
      (Variables|Default|SetRightPosOffset _openoffset)
      (Variables|Default|SetLeftPosOffset (* _openoffset -1.0)))))

(fn Close
  (bind _result (Math|Integer|DecrementInt (Variables|Default|GetOpenCounter))
    (:%20%20
      (if (== _result 0)
        (Variables|Default|SetLeftPosOffset 0.0)
        (Variables|Default|SetRightPosOffset 0.0)))))