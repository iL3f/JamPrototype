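; Lift actor that shuttles between two target points, A and B, pausing for WaitTime at each end.
; BeginPlay heads it toward point A and prints an error for unset points, though A is read before that check.
; Tick steps it by up to MoveSpeed per frame without delta-time scaling.
; On arrival, ReachTime guards a single Delay before StartMove clears it and switches the target to the opposite point.
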(event EventBeginPlay
  (bind _self self)
  (bind _returnvalue (Utilities|GetDisplayName _self))
  (Variables|Default|SetTargetPosition (Transformation|GetActorLocation (Variables|Default|GetTargetPointA)))
  (Utilities|FlowControl|Sequence
    (:then_0
      (Utilities|IsValid (Variables|Default|GetTargetPointA)
        (:Is%20Not%20Valid
          (Development|PrintString (Utilities|String|Append "You must set target point A for " _returnvalue)))))
    (:then_1
      (Utilities|IsValid (Variables|Default|GetTargetPointB)
        (:Is%20Not%20Valid
          (Development|PrintString (Utilities|String|Append "You must set target point B for " _returnvalue)))))))

(event EventTick
  (params (DeltaSeconds :type Float%20%28single-precision%29))
  (bind _returnvalue (Transformation|GetActorLocation))
  (bind _targetposition (Variables|Default|GetTargetPosition))
  (bind _returnvalue_2 (- _targetposition _returnvalue))
  (Transformation|SetActorLocation (+ _returnvalue (* (Math|Vector|Normalize _returnvalue_2) (Math|Float|Min(Float) (Math|Vector|VectorLength _returnvalue_2) (Variables|Default|GetMoveSpeed)))) false false)
  (if (Math|Vector|Equal(Vector) _returnvalue _targetposition 1.0)
    (if (== (Variables|Default|GetReachTime) 0.0)
      (Variables|Default|SetReachTime (Actor|GetGameTimeSinceCreation))
      (Utilities|FlowControl|Delay (Variables|Default|GetWaitTime))
      (CallFunction|StartMove))))

(event Collision|EventActorBeginOverlap
  (params (OtherActor :type Actor%20Object%20Reference)))

(fn ConstructionScript)

(fn StartMove
  (bind _targetpointa (Variables|Default|GetTargetPointA))
  (bind _targetpointb (Variables|Default|GetTargetPointB))
  (bind _returnvalue (Transformation|GetActorLocation _targetpointa))
  (bind _returnvalue_2 (Transformation|GetActorLocation _targetpointb))
  (Variables|Default|SetReachTime 0.0)
  (if (CallFunction|IsatPoint _returnvalue)
    (Variables|Default|SetTargetPosition _returnvalue_2)
    (elif (CallFunction|IsatPoint _returnvalue_2)
      (Variables|Default|SetTargetPosition _returnvalue))))

(fn IsatPoint
  (params (Point :type Vector))
  (return (Math|Vector|Equal(Vector) Point (Transformation|GetActorLocation) 1.0)))