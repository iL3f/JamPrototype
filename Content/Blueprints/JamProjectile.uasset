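; JamProjectile is a projectile actor that damages what it hits.
; On BeginPlay it binds a handler to its sphere collision's component hit event.
; The handler applies DamageAmount through the hit actor's JamDamagable component, skipping its owner and actors without that component.
; The projectile destroys itself on any hit, whether or not damage is dealt.
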(event Custom|Hit
  (params (HitComponent :type Primitive%20Component%20Object%20Reference) (OtherActor :type Actor%20Object%20Reference) (OtherComp :type Primitive%20Component%20Object%20Reference) (NormalImpulse :type Vector) (Hit :type Hit%20Result%20Structure%20%28by%20ref%29))
  (bind _returnvalue (Actor|GetComponentbyClass OtherActor "/Game/Blueprints/JamDamagable.JamDamagable_C"))
  (if (and (Utilities|IsValid OtherActor) (!= OtherActor (Components|GetOwner)))
    (Utilities|IsValid _returnvalue
      (:Is%20Valid
        (Default|Damage _returnvalue (Variables|Default|GetDamageAmount)))
      (:Is%20Not%20Valid
        _)))
  (Actor|DestroyActor))

(event EventBeginPlay
  (Collision|BindEventtoOnComponentHit (Variables|Default|GetSphereCollision) (delegate Custom|Hit)))

(fn ConstructionScript)