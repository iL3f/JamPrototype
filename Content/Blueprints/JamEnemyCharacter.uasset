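; Enemy character Blueprint that patrols between points and ragdolls on death, working with a JamAiController.
; GoToNextPoint cycles through the PatrolPoints array with wraparound and passes the current point to the controller.
; When the JamDamagable component reports death, it switches the mesh to ragdoll physics, disables capsule collision and movement, then notifies the controller.
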(event Custom|Dead
  (CallFunction|StartRagdoll)
  (bind _asjam_ai_controller (Utilities|Casting|CastToJamAiController (Pawn|GetController)))
  (Default|OnDied _asjam_ai_controller))

(event EventBeginPlay
  (EventDispatchers|AssignOnDead (Variables|Default|GetJamDamagable) (delegate Custom|Dead)))

(fn ConstructionScript)

(fn GotoNextPoint
  (bind _patrolpoints (Variables|Default|GetPatrolPoints))
  (bind _returnvalue (Utilities|Array|Length _patrolpoints))
  (if (!= _returnvalue 0)
    (bind _output_get (Variables|Default|SetCurrentPatrolPoint (Math|Integer|%(Integer) (+ (Variables|Default|GetCurrentPatrolPoint) 1) _returnvalue)))
    (LocalVariables|SetPatrolPoint (Utilities|Array|Get(acopy) (Variables|Default|GetPatrolPoints) _output_get)))
  (bind _asjam_ai_controller (Utilities|Casting|CastToJamAiController (Pawn|GetController)))
  (Default|SetPatrolPoint _asjam_ai_controller (LocalVariables|GetPatrolPoint)))

(fn StartRagdoll
  (bind _mesh (Variables|Character|GetMesh))
  (bind _charactermovement (Variables|Character|GetCharacterMovement))
  (Physics|SetSimulatePhysics _mesh true)
  (Collision|SetCollisionProfileName _mesh "Ragdoll" :!class /Script/Engine.PrimitiveComponent)
  (Collision|SetCollisionResponsetoAllChannels (Variables|Collision|GetCapsuleComponent) "ECR_Ignore")
  (Components|Movement|StopMovementImmediately _charactermovement)
  (Pawn|Components|CharacterMovement|DisableMovement _charactermovement)
  (Components|Tick|SetComponentTickEnabled _charactermovement false))