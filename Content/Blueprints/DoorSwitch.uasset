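; DoorSwitch is an interactable switch actor that sets the state of a linked Door.
; Overlapping JamCharacters controlled by a PlayerController get input enabled on the switch, which is disabled again when they leave.
; Pressing Interact while input is enabled passes the EnableDoor value to SetDoorState on the Door reference, if it is valid.
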(event EventBeginPlay)

(event Collision|EventActorBeginOverlap
  (params (OtherActor :type Actor%20Object%20Reference))
  (bind _asjam_character (Utilities|Casting|CastToJamCharacter OtherActor))
  (bind _asplayer_controller (Utilities|Casting|CastToPlayerController (Pawn|GetController _asjam_character)))
  (Input|EnableInput _asplayer_controller))

(event Collision|EventActorEndOverlap
  (params (OtherActor :type Actor%20Object%20Reference))
  (bind _asjam_character (Utilities|Casting|CastToJamCharacter OtherActor))
  (bind _asplayer_controller (Utilities|Casting|CastToPlayerController (Pawn|GetController _asjam_character)))
  (Input|DisableInput _asplayer_controller))

(event Input|ActionEvents|InputActionInteract
  (params (Key :type Key%20Structure))
  (bind _door (Variables|Default|GetDoor))
  (:Pressed
    (Utilities|IsValid _door
      (:Is%20Valid
        (Default|SetDoorState _door (Variables|Default|GetEnableDoor))))))

(fn ConstructionScript)